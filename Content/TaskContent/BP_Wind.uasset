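; BP_Wind is a wind zone actor that pushes the player character while it stands inside a box volume.
; A looping half-second timer checks the box's overlapping actors and launches the player along WindDirection scaled by WindStrength, adding to existing velocity.
; The construction script picks a dust or mist Niagara effect and passes the same direction and strength to it, so the visuals follow the push settings.
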(event `self.ReceiveBeginPlay`
  (`KismetSystemLibrary.K2_SetTimerDelegate` (delegate `WindForce`) 0.5 true))

(event `WindForce`
  (bind _returnvalue (`GameplayStatics.GetPlayerCharacter` 0))
  (for _array_element (`PrimitiveComponent.GetOverlappingActors` (`self.Box`) null)
    (if (== _array_element _returnvalue)
      (`Character.LaunchCharacter` _returnvalue (* (`self.WindDirection`) (`self.WindStrength`)) false false))))

(fn `UserConstructionScript`
  (switch `string` (`self.ParticleAsset`)
    (:`Wind_Dust`
      (`NiagaraComponent.SetAsset` (`self.Niagara`) "/Game/TaskContent/DustParticles.DustParticles" true))
    (:`Wind_Mist`
      (`NiagaraComponent.SetAsset` (`self.Niagara`) "/Game/TaskContent/MistParticles.MistParticles" true)))
  (`NiagaraComponent.SetNiagaraVariableVec3` (`self.Niagara`) "WindDirection" (`self.WindDirection`))
  (`NiagaraComponent.SetNiagaraVariableFloat` (`self.Niagara`) "WindSpeedUser" (`self.WindStrength`)))