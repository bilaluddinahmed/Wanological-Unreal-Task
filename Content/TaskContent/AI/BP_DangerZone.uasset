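; BP_DangerZone is a spherical trigger actor that tells the enemy AI when the player enters or leaves a danger zone.
; The construction script sizes the sphere from a Radius variable, and BeginPlay caches a single BP_EnemyAI found with GetActorOfClass.
; Overlap events filter for the player character, print a debug string, and call the entered or exited message on that AI.
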(event `self.ReceiveBeginPlay`
  (bind _returnvalue (`GameplayStatics.GetActorOfClass` "/Game/TaskContent/AI/BP_EnemyAI.BP_EnemyAI_C"))
  (set `self.EnemyAI` _returnvalue))

(event `self.ReceiveActorBeginOverlap`
  (params (OtherActor :type "Actor Object Reference"))
  (if (== OtherActor (`GameplayStatics.GetPlayerCharacter` 0))
    (`KismetSystemLibrary.PrintString` "Entered" true true (struct :`R` 0.092601 :`G` 1.0 :`A` 1.0))
    (message `/Game/TaskContent/AI/BPI_DangerZone.EnteredDZ` (`self.EnemyAI`))))

(event `self.ReceiveActorEndOverlap`
  (params (OtherActor :type "Actor Object Reference"))
  (if (== OtherActor (`GameplayStatics.GetPlayerCharacter` 0))
    (`KismetSystemLibrary.PrintString` "Exited" true true (struct :`G` 0.027267 :`B` 1.0 :`A` 1.0))
    (message `/Game/TaskContent/AI/BPI_DangerZone.ExitedDZ` (`self.EnemyAI`))))

(fn `UserConstructionScript`
  (`SphereComponent.SetSphereRadius` (`self.Sphere`) (`self.Radius`) true))